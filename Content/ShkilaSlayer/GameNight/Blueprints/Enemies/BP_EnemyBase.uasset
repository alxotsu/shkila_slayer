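; BP_EnemyBase is an enemy base Blueprint for the GameNight mode, with health and pawn sensing.
; An ApplyDamage event subtracts damage from Health and destroys the actor at zero or below.
; PawnSensing casts seen pawns to BP_PawnNight but does nothing further, as the node setting the TargetActor blackboard key is never executed.
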(event `/Game/ShkilaSlayer/GameNight/Blueprints/Enemies/BPI_Damagable.ApplyDamage`
  (params (damage :type "Float (double-precision)"))
  (bind _output_get (set `self.Health` (- (`self.Health`) damage)))
  (if (<= _output_get 0.0)
    (`self.K2_DestroyActor`)))

(event `self.PawnSensing.OnSeePawn`
  (params (Pawn :type "Pawn Object Reference"))
  (bind _asbp_pawn_night (cast `/Game/ShkilaSlayer/GameNight/Blueprints/Player/BP_PawnNight` Pawn)))

(fn `UserConstructionScript`)