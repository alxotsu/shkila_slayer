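; Base falling-object actor that takes its fall speed from BP_GameMode and registers itself in that game mode's SpawnedObjects list.
; A fast looping timer, rather than Tick, runs Move to lower RenderComponent with a swept move by a fixed step per call.
; The actor destroys itself below a hard-coded height, as a workaround for Kill Z not working, and removes itself from the list when destroyed.
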(event `self.ReceiveBeginPlay`
  (`|ExecutionSequence`
    (:`then_0`
      (bind _asbp_game_mode (cast `/Game/T01/blueprints/Game/BP_GameMode` (`GameplayStatics.GetGameMode`)))
      (set `self.fallSpeed` (`/Game/T01/blueprints/Game/BP_GameMode.ObjectFallSpeed` _asbp_game_mode)))
    (:`then_1`
      (bind _asbp_game_mode_2 (cast `/Game/T01/blueprints/Game/BP_GameMode` (`GameplayStatics.GetGameMode`)))
      (`BlueprintSetLibrary.Set_Add` (`/Game/T01/blueprints/Game/BP_GameMode.SpawnedObjects` _asbp_game_mode_2) self))
    (:`then_2`
      (bind _returnvalue (`KismetSystemLibrary.K2_SetTimerDelegate` (delegate `Event Move`) 0.01 true))
      (setmembers `TimerHandle` :`StructRef` _returnvalue))))

(event `Event Move`
  (bind _rendercomponent (`self.RenderComponent`))
  (bind _returnvalue (- (.z (`SceneComponent.K2_GetComponentLocation` _rendercomponent)) (`self.fallSpeed`)))
  (`SceneComponent.K2_SetWorldLocation` _rendercomponent (`KismetMathLibrary.MakeVector` (.x (`SceneComponent.K2_GetComponentLocation` _rendercomponent)) (.y (`SceneComponent.K2_GetComponentLocation` _rendercomponent)) _returnvalue) true false)
  (if (< _returnvalue -1000.0)
    (`self.K2_DestroyActor`)))

(event `self.ReceiveDestroyed`
  (bind _asbp_game_mode (cast `/Game/T01/blueprints/Game/BP_GameMode` (`GameplayStatics.GetGameMode`)))
  (`BlueprintSetLibrary.Set_Remove` (`/Game/T01/blueprints/Game/BP_GameMode.SpawnedObjects` _asbp_game_mode) self))

(fn `UserConstructionScript`)